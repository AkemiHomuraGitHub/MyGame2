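; Base character Blueprint for combat units that chase an enemy, attack within range and die when health runs out.
; BattleBehavior, not called here, takes its target from FindClosestEnemy, an empty stub in this class, then triggers attack or simple move-to events by distance.
; One montage supplies Attack and Dead sections, with a DoOnce reset after an AttackRate delay throttling attacks.
; AnyDamage reduces health, and death destroys the actor once its montage completes.
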(event Custom|AttackEvent
  (Utilities|IsValid (Variables|Value|GetEnemy)
    (:Is%20Valid
      (Utilities|FlowControl|DoOnce false :!label _label
        (:Completed
          (Animation|Montage|PlayMontage (Variables|Character|GetMesh self) (Variables|Init|GetMyMontage) 1.0 0.0 "Attack"
            (:then
              (Utilities|FlowControl|Delay (Variables|Attribute|GetAttackRate))
              (goto _label Reset))))))
    (:Is%20Not%20Valid
      (Development|PrintString "Enemy is not valid"))))

(event Custom|MoveEvent
  (params (Pos :type Vector))
  (AI|Navigation|SimpleMovetoLocation 0 Pos))

(event Custom|StopEvent
  (params (Complete :type Boolean))
  (if Complete
    (Animation|StopAnimMontage (Variables|Init|GetMyMontage)))
  (Components|Movement|StopMovementImmediately (Variables|Character|GetCharacterMovement)))

(event Custom|DeadEvent
  (Animation|Montage|PlayMontage (Variables|Character|GetMesh self) (Variables|Init|GetMyMontage) 1.0 0.0 "Dead"
    (:OnCompleted
      (Actor|DestroyActor))))

(event EventBeginPlay)

(event Collision|EventActorBeginOverlap
  (params (OtherActor :type Actor%20Object%20Reference)))

(event EventTick
  (params (DeltaSeconds :type Float%20%28single-precision%29)))

(event Game|Damage|EventAnyDamage
  (params (Damage :type Float%20%28single-precision%29) (DamageType :type Damage%20Type%20Object%20Reference) (InstigatedBy :type Controller%20Object%20Reference) (DamageCauser :type Actor%20Object%20Reference))
  (Behavior|GetDamage Damage))

(fn ConstructionScript)

(fn InRange
  (return (<= (Function|DisfromEnemy) (Variables|Attribute|GetRange))))

(fn DisfromEnemy
  (if (Utilities|IsValid (Variables|Value|GetEnemy))
    (return (Math|Vector|VectorLength (- (Transformation|GetActorLocation (Variables|Value|GetEnemy)) (Transformation|GetActorLocation self))))
    (else
      (return 1e+04))))

(fn BattleBehavior
  (bind _enemy (函数|FindClosestEnemy))
  (if (Variables|State|GetIsAttack?)
    (Utilities|IsValid _enemy
      (:Is%20Valid
        (Variables|Value|SetEnemy _enemy)
        (if (函数|InRange)
          (CallFunction|AttackEvent)
          (else
            (CallFunction|MoveEvent (Transformation|GetActorLocation (Variables|Value|GetEnemy)))))))))

(fn FindClosestEnemy
  (return 0))

(fn GetDamage
  (params (Damage :type Float%20%28single-precision%29))
  (Variables|Attribute|SetHealth (Math|Float|Max(Float) (- (Variables|Attribute|GetHealth) Damage) 0.0))
  (if (<= (Variables|Attribute|GetHealth) 0.1)
    (CallFunction|DeadEvent)))