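; BP_Hero is a hero character Blueprint that automatically targets nearby enemies and chases or attacks them.
; Every tick, FindClosestEnemy scans all BP_CharacterBase actors tagged "Enemy" within a fixed radius and keeps the closest, never clearing the previous target.
; While IsAttack is set and the target is valid, it calls AttackEvent when in range, otherwise MoveEvent toward the enemy's location.
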(event EventBeginPlay
  (|CallParentFunction))

(event Collision|EventActorBeginOverlap
  (params (OtherActor :type Actor%20Object%20Reference))
  (|CallParentFunction OtherActor) ; 此节点被禁用，将不会被调用。\n从引脚连出引线来编译功能。
)

(event EventTick
  (params (DeltaSeconds :type Float%20%28single-precision%29))
  (|CallParentFunction DeltaSeconds)
  (CallFunction|FindClosestEnemy)
  (Utilities|IsValid (Variables|Default|GetEnemy)
    (:Is%20Valid
      (if (Variables|Default|GetIsAttack? self)
        (if (CallFunction|InRange)
          (CallFunction|AttackEvent)
          (else
            (CallFunction|MoveEvent (Transformation|GetActorLocation (Variables|Default|GetEnemy)))))))))

(fn ConstructionScript
  (|CallParentFunction))

(fn FindClosestEnemy
  (bind _outactors (Actor|GetAllActorsOfClass "/Game/BluePrints/Character/BP_CharacterBase.BP_CharacterBase_C"))
  (for _array_element _outactors
    (if (Actor|ActorHasTag _array_element "Enemy")
      (if (<= (CallFunction|DisfromActor _array_element) 1e+03)
        (Utilities|IsValid (Variables|Default|GetEnemy)
          (:Is%20Valid
            (if (>= (CallFunction|DisfromEnemy) (CallFunction|DisfromActor _array_element))
              (Variables|Default|SetEnemy _array_element)))
          (:Is%20Not%20Valid
            (Variables|Default|SetEnemy _array_element))))))
  (return))