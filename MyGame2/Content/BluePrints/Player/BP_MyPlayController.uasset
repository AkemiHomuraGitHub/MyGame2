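; Player controller for MOBA-style mouse control of a Hero with an edge-scrolling camera pawn.
; Right click sends the Hero to the point under the cursor through MoveEvent.
; AttackKey arms attack mode with a hand cursor; left click then flags IsAttack and moves the Hero, and release restores the default cursor.
; Each tick, CamMove shifts the possessed BP_MyPawn when the mouse nears a viewport edge.
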(event EventBeginPlay
  (bind _asbp_my_pawn (Utilities|Casting|CastToBP_MyPawn (Pawn|GetControlledPawn self)))
  (Variables|Character|SetMyPawn _asbp_my_pawn))

(event EventTick
  (params (DeltaSeconds :type Float%20%28single-precision%29))
  (Behavior|CamMove))

(event Input|ActionEvents|InputActionAttackKey
  (params (Key :type Key%20Structure :default "None"))
  (:Pressed
    (Development|PrintString "Hello")
    (Variables|Value|SetSetA true)
    (Variables|Default|SetCurrentMouseCursor "Hand")))

(event Input|MouseEvents|LeftMouseButton
  (params (Key :type Key%20Structure :default "None"))
  (:Pressed
    (if (Variables|Value|GetSetA)
      (Variables|/Game/BluePrints/Character/BP_CharacterBase.BP_CharacterBase_C|SetIsAttack? (Variables|Character|GetHero) true)
      (Default|MoveEvent (Variables|Character|GetHero) (Function|GetMousePos))))
  (:Released
    (Variables|Value|SetSetA false)
    (Variables|Default|SetCurrentMouseCursor "Default")))

(event Input|MouseEvents|RightMouseButton
  (params (Key :type Key%20Structure :default "None"))
  (:Pressed
    (Default|MoveEvent (Variables|Character|GetHero) (Function|GetMousePos))))

(fn ConstructionScript)

(fn CamMove
  (bind (_locationx _locationy) (Game|Player|GetMousePosition))
  (bind (_sizex _sizey) (HUD|GetViewportSize))
  (bind _returnvalue (Math|Conversions|ToFloat(Integer) _sizex))
  (bind _returnvalue_2 (Math|Conversions|ToFloat(Integer) _sizey))
  (bind _returnvalue_3 (/ _locationx _returnvalue))
  (bind _returnvalue_4 (/ _locationy _returnvalue_2))
  (Class|Actor|AddActorLocalTransform (Variables|Character|GetMyPawn) (Math|Conversions|ToTransform(Vector) (+ (+ (Math|Vector|SelectVector "0.000000,20.000000,0.000000" "0.000000, 0, 0" (>= _returnvalue_3 0.95)) (Math|Vector|SelectVector "0.000000,-20.000000, 0" "0, 0, 0" (<= _returnvalue_3 0.05))) (+ (Math|Vector|SelectVector "-20.000000,0.000000, 0" "0, 0, 0" (>= _returnvalue_4 0.95)) (Math|Vector|SelectVector "20.000000,0.000000, 0" "0, 0, 0" (<= _returnvalue_4 0.05))))) false false))

(fn GetMousePos
  (return (.Location (Collision|BreakHitResult (.HitResult (Game|Player|GetHitResultUnderCursorbyChannel "TraceTypeQuery1" true))))))